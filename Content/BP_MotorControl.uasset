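; Motor control test Blueprint that talks to SimCorDX motion software on localhost over a UDP sender using the ObjectDeliverer plugin.
; BeginPlay sends an ID string, then Tick streams a fixed zero-valued "~M" motion command.
; Held D and A keys step a clamped Speed up or down.
; Tick uses Speed as timeline time to derive SmoothSpeed, which is only printed, never sent.
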(event `self.ReceiveBeginPlay`
  (bind _returnvalue (`KismetStringLibrary.Concat_StrStr` "#id" "CinematicExperience" "\\n"))
  (`self.EnableInput` (`GameplayStatics.GetPlayerController` 0))
  (bind _output_get (set `self.DelivMangr` (`ObjectDelivererManager.CreateObjectDelivererManager` true)))
  (add `ObjectDelivererManager.Connected` _output_get (delegate `Connected`))
  (add `ObjectDelivererManager.Disconnected` (`self.DelivMangr`) (delegate `DIsconnected`))
  (bind _output_get_2 (set `self.DelivBox` (`DeliveryBoxFactory.CreateUtf8StringDeliveryBox`)))
  (add `Utf8StringDeliveryBox.Received` _output_get_2 (delegate `Recieved`))
  (`ObjectDelivererManager.Start` (`self.DelivMangr`) (`ProtocolFactory.CreateProtocolUdpSocketSender` "127.0.0.1" 1288) (`PacketRuleFactory.CreatePacketRuleNodivision`) (`self.DelivBox`))
  (`Utf8StringDeliveryBox.Send` (`self.DelivBox`) _returnvalue)
  (`KismetSystemLibrary.PrintString` _returnvalue)
  (`KismetSystemLibrary.Delay` 0.3))

(event `Connected`
  (params (ClientSocket :type "ObjectDelivererProtocol Object Reference"))
  (`KismetSystemLibrary.PrintString` "Connected to SimCorDX!"))

(event `DIsconnected`
  (params (ClientSocket :type "ObjectDelivererProtocol Object Reference"))
  (`KismetSystemLibrary.PrintString` "Disconnected to SimCorDX!"))

(event `Recieved`
  (params (ReceivedString :type String) (FromObject :type "ObjectDelivererProtocol Object Reference"))
  (`KismetSystemLibrary.PrintString` (`KismetStringLibrary.Concat_StrStr` "SimCoreDX says:" ReceivedString)))

(event `self.ReceiveTick`
  (params (DeltaSeconds :type "Float (single-precision)"))
  (bind _returnvalue (`GameplayStatics.GetWorldDeltaSeconds`))
  (bind _speed (`self.speed`))
  (bind _returnvalue_2 (`KismetStringLibrary.Concat_StrStr` "~M" "0 0 0 " (`KismetStringLibrary.Concat_StrStr` "0 " (`KismetStringLibrary.Conv_DoubleToString` 0.0) "0 ")))
  (`Utf8StringDeliveryBox.Send` (`self.DelivBox`) _returnvalue_2)
  (`KismetSystemLibrary.PrintString` _returnvalue_2)
  (if (> _speed 0.0)
    (bind (_direction _newtrack_0) (`Timeline|Timeline_Smooth` :`NewTime` _speed :!via `SetNewTime`)
      (:`Update`
        (set `self.SmoothSpeed` _newtrack_0)))
    (else
      (bind (_direction_2 _newtrack_0_2) (`Timeline|Timeline_1` :`NewTime` (* _speed -1.0) :!via `SetNewTime`)
        (:`Update`
          (bind _output_get (set `self.SmoothSpeed` (* _newtrack_0_2 -1.0)))))))
  (`KismetSystemLibrary.PrintString` (`KismetStringLibrary.Conv_DoubleToString` _output_get) true true (struct :`R` 0.280722 :`G` 1.0 :`B` 0.43803 :`A` 1.0) _returnvalue)
  (`KismetSystemLibrary.PrintString` (`KismetStringLibrary.Conv_DoubleToString` (`self.speed`)) true true (struct :`G` 0.66 :`B` 1.0 :`A` 1.0) _returnvalue))

(event `epickey`
  (bind _speed (`self.speed`))
  (set `self.turning right` true :!label _label)
  (if (`self.turning right`) :!label _label_2
    ;[1 1 1] Clamp
    (set `self.speed` (+ _speed 0.1))
    (if (> _speed 1.0)
      (set `self.speed` 1.0))
    (`KismetSystemLibrary.Delay` 0.1)
    (goto _label_2)))

(event `Key|D`
  (params (Key :type "Key Structure"))
  (:`Pressed`
    (goto _label))
  (:`Released`
    (set `self.turning right` false)))

(event `Key|A`
  (params (Key :type "Key Structure"))
  (bind _speed (`self.speed`))
  (:`Pressed`
    (set `self.Trning Left` true)
    (if (`self.Trning Left`) :!label _label_3
      ;[1 1 1] Clamp
      (set `self.speed` (+ _speed -0.1))
      (if (< _speed -1.0)
        (set `self.speed` -1.0)
        (else
          (`KismetSystemLibrary.Delay` 0.1)
          (goto _label_3)))))
  (:`Released`
    (set `self.Trning Left` false)))

(fn `UserConstructionScript`)